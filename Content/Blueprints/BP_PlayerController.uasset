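; Player controller that lets one player switch between Warrior, Wizard and Rogue pawns moving along the X axis.
; BeginPlay orders the placed pawns into a fixed array, creates gameplay and pause widgets, and possesses after a delay; swapping cycles possession and updates the portrait.
; Inputs reach pawns through movement calls and interface messages, gated by ability and interaction state.
; It also handles pausing and broadcasts keyboard or gamepad control changes.
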(event Custom|ResumeGame
  (Game|SetGamePaused false)
  (Variables|Default|SetbShowMouseCursor false)
  (Input|SetInputModeGameOnly self))

(event EventBeginPlay
  (bind _currentcharacterindex (Variables|Default|GetCurrentCharacterIndex))
  (bind _outactors (Actor|GetAllActorsOfClass "/Game/Blueprints/BP_CharacterPawn.BP_CharacterPawn_C"))
  (bind _orderedarray (CallFunction|ReorderCharacterArray _outactors))
  (Variables|Default|SetCharacters _orderedarray)
  (bind _returnvalue (UserInterface|CreateWidget "/Game/Widgets/W_Gameplay.W_Gameplay_C"))
  (Variables|Default|SetGameplayWidget _returnvalue)
  (UserInterface|Viewport|AddtoViewport (Variables|Default|GetGameplayWidget) 0)
  (bind _outactors_2 (Actor|GetAllActorsOfClass "/Script/Engine.CameraActor"))
  (Actor|DestroyActor (Utilities|Array|Get(acopy) _outactors_2))
  (Default|UpdateSelectedPortrait (Variables|Default|GetGameplayWidget) _currentcharacterindex)
  (Utilities|FlowControl|Delay 1.5)
  (Pawn|Possess (Utilities|Array|Get(acopy) (Variables|Default|GetCharacters) _currentcharacterindex))
  (bind _returnvalue_2 (UserInterface|CreateWidget "/Game/Widgets/W_PauseMenu.W_PauseMenu_C" (Game|GetPlayerController 0)))
  (bind _output_get (Variables|Default|SetPauseMenu _returnvalue_2))
  (EventDispatchers|BindEventtoOnRemovefromViewport _output_get (delegate Custom|ResumeGame)))

(event EventTick
  (params (DeltaSeconds :type Float%20%28single-precision%29)))

(event Input|ActionEvents|InputActionJump
  (params (Key :type Key%20Structure :default "None"))
  (bind _returnvalue (Pawn|GetControlledPawn))
  (:Pressed
    (bind _isusingability (CallFunction|IsPawnUsingAbility))
    (if (and (not _isusingability) (not (Variables|Default|GetIsInteracting)))
      (bind _ascharacter (Utilities|Casting|CastToCharacter _returnvalue))
      (Class|BPIFlipbook|ApplyForce(Message) _ascharacter)
      (Character|Jump _ascharacter)))
  (:Released
    (bind _isusingability_2 (CallFunction|IsPawnUsingAbility))
    (if (and (not _isusingability_2) (not (Variables|Default|GetIsInteracting)))
      (bind _ascharacter_2 (Utilities|Casting|CastToCharacter _returnvalue))
      (Character|StopJumping _ascharacter_2))))

(event Input|ActionEvents|InputActionSwapCharacters
  (params (Key :type Key%20Structure :default "None"))
  (:Pressed
    (if (not (Variables|Default|GetIsInteracting))
      (bind _result (Math|Integer|IncrementInt (Variables|Default|GetCurrentCharacterIndex))
        (:%20%20
          (if (>= _result (Utilities|Array|Length (Variables|Default|GetCharacters)))
            (Variables|Default|SetCurrentCharacterIndex 0))
          (Pawn|Possess (Utilities|Array|Get(acopy) (Variables|Default|GetCharacters) (Variables|Default|GetCurrentCharacterIndex)))
          (Default|UpdateSelectedPortrait (Variables|Default|GetGameplayWidget) (Variables|Default|GetCurrentCharacterIndex)))))))

(event Input|ActionEvents|InputActionUseAbility
  (params (Key :type Key%20Structure :default "None"))
  (:Pressed
    (bind _canuse (CallFunction|CanPawnUseAbility))
    (if (and _canuse (not (Variables|Default|GetIsInteracting)))
      (Class|BPIFlipbook|UseAbility(Message) (Pawn|GetControlledPawn)))))

(event Input|ActionEvents|InputActionInteract
  (params (Key :type Key%20Structure :default "None"))
  (:Pressed
    (Class|BPIFlipbook|InteractwithInteractable(Message) (Pawn|GetControlledPawn))))

(event Input|ActionEvents|InputActionPause
  (params (Key :type Key%20Structure :default "None"))
  (bind _pausemenu (Variables|Default|GetPauseMenu))
  (:Pressed
    (if (and (not (Game|IsGamePaused)) (!= (Variables|Default|GetPauseMenu) 0))
      (Default|AddtoView _pausemenu)
      (Input|SetInputModeUIOnly self _pausemenu "DoNotLock")
      (Variables|Default|SetbShowMouseCursor true)
      (Game|SetGamePaused true))))

(event Input|AxisEvents|InputAxisMoveRight
  (params (AxisValue :type Float%20%28single-precision%29))
  (bind _isusingability (CallFunction|IsPawnUsingAbility))
  (bind _canuse (CallFunction|CanPawnUseAbility))
  (if (Math|Boolean|ANDBoolean (not _isusingability) _canuse (not (Variables|Default|GetIsInteracting)))
    (if (> AxisValue 0.0)
      (Class|BPIFlipbook|LookRight(Message) (Pawn|GetControlledPawn))
      (CallFunction|ApplyMovementtoPawn AxisValue))))

(event Input|AxisEvents|InputAxisMoveLeft
  (params (AxisValue :type Float%20%28single-precision%29))
  (bind _isusingability (CallFunction|IsPawnUsingAbility))
  (bind _canuse (CallFunction|CanPawnUseAbility))
  (if (Math|Boolean|ANDBoolean _canuse (not _isusingability) (not (Variables|Default|GetIsInteracting)))
    (if (< AxisValue 0.0)
      (Class|BPIFlipbook|LookLeft(Message) (Pawn|GetControlledPawn))
      (CallFunction|ApplyMovementtoPawn AxisValue))))

(event Input|KeyboardEvents|AnyKey
  (params (Key :type Key%20Structure :default "None"))
  (:Pressed
    (if (Class|KismetInputLibrary|KeyIsGamepadKey Key)
      (Variables|Default|SetGameplayControls "NewEnumerator1")
      (else
        (Variables|Default|SetGameplayControls "NewEnumerator0")))
    (Default|CallOnGameplayControlChange (Variables|Default|GetGameplayControls))))

(fn ConstructionScript)

(fn ApplyMovementtoPawn
  (params (AxisValue :type Float%20%28double-precision%29))
  (Pawn|Input|AddMovementInput (Pawn|GetControlledPawn) "1.000000, 0, 0" (/ AxisValue 3.0) false))

(fn ReorderCharacterArray
  (params (CharacterArray :type Array%20of%20BP%20Character%20Pawn%20Object%20References))
  (Utilities|Array|Resize (LocalVariables|Getlocal_orderedArray) 3)
  (for _array_element CharacterArray
    (bind _asbp_warrior (Utilities|Casting|CastToBP_Warrior _array_element)
      (:then
        (Utilities|Array|SetArrayElem (LocalVariables|Getlocal_orderedArray) 0 _asbp_warrior))
      (:CastFailed
        (bind _asbp_wizard (Utilities|Casting|CastToBP_Wizard _array_element)
          (:then
            (Utilities|Array|SetArrayElem (LocalVariables|Getlocal_orderedArray) 1 _asbp_wizard))
          (:CastFailed
            (bind _asbp_rogue (Utilities|Casting|CastToBP_Rogue _array_element))
            (Utilities|Array|SetArrayElem (LocalVariables|Getlocal_orderedArray) 2 _asbp_rogue))))))
  (return (LocalVariables|Getlocal_orderedArray)))

(fn IsPawnUsingAbility
  (bind _isusingability (Class|BPIFlipbook|IsAbilityActive(Message) (Pawn|GetControlledPawn)))
  (return _isusingability))

(fn CanPawnUseAbility
  (bind _canuse (Class|BPIFlipbook|CanUseAbility(Message) (Pawn|GetControlledPawn)))
  (return _canuse))