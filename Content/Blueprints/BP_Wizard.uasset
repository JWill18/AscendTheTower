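; BP_Wizard is a wizard actor whose ability casts a spell projectile.
; UseAbility calls the parent implementation and plays a fireball cast sound.
; Tick spawns BP_WizardProjectile at SpellSpawn once the Wizard_Ability flipbook passes a set fraction of its length, timing the shot to the animation without a notify.
; An accumulated timer, reset on each spawn and checked against AbilityTimer, prevents repeat spawns during the same animation.
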(event EventBeginPlay
  (|CallParentFunction) ; This node is disabled and will not be called.\nDrag off pins to build functionality.
)

(event Collision|EventActorBeginOverlap
  (params (OtherActor :type Actor%20Object%20Reference))
  (|CallParentFunction OtherActor) ; This node is disabled and will not be called.\nDrag off pins to build functionality.
)

(event EventTick
  (params (DeltaSeconds :type Float%20%28single-precision%29))
  (bind _sprite (Variables|Default|GetSprite))
  (|CallParentFunction DeltaSeconds)
  ;[1 1 1] Used to prevent spawning another one before the animation ends
  (Variables|Default|SetCurrentAbilityTimer (+ (Variables|Default|GetCurrentAbilityTimer) DeltaSeconds))
  (if (and (and (== (Class|PaperFlipbookComponent|GetFlipbook _sprite) "/Game/AssetPacks/Characters/Wizard_Pack/Wizard_Pack/Ability/Wizard_Ability.Wizard_Ability") (> (/ (Math|Conversions|ToFloat(Integer) (Class|PaperFlipbookComponent|GetPlaybackPositioninFrames _sprite)) (Math|Conversions|ToFloat(Integer) (Class|PaperFlipbookComponent|GetFlipbookLengthinFrames _sprite))) 0.7)) (>= (Variables|Default|GetCurrentAbilityTimer) (Variables|Default|GetAbilityTimer)))
    (Game|SpawnActorfromClass "/Game/Blueprints/BP_WizardProjectile.BP_WizardProjectile_C" (Transformation|GetWorldTransform (Variables|Default|GetSpellSpawn)) "Undefined" 0 0)
    (Variables|Default|SetCurrentAbilityTimer 0.0)))

(event EventUseAbility
  (|CallParentFunction)
  (Audio|PlaySound2D "/Game/Assets/Sounds/334237__liamg-sfx__fireball-cast-3.334237__liamg-sfx__fireball-cast-3" 1.0 1.0 0.0 0 0))

(fn ConstructionScript
  (|CallParentFunction))