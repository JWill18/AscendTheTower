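; BP_Barricade is a breakable 2D barricade that plays a breakdown animation and then removes itself.
; Break runs once, guarded by IsBreaking, swapping the Paper2D flipbook to the non-looping BoxBreakdown and playing a crate-break sound.
; The flipbook's OnFinishedPlaying event destroys the actor, so its lifetime follows the animation rather than a timer.
; Nothing in this Blueprint calls Break, so it relies on an external trigger.
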(event OnFinishedPlaying(PaperFlipbook)
  (Actor|DestroyActor))

(event EventBeginPlay)

(event Collision|EventActorBeginOverlap
  (params (OtherActor :type Actor%20Object%20Reference)))

(event EventTick
  (params (DeltaSeconds :type Float%20%28single-precision%29)))

(fn ConstructionScript)

(fn Break
  (bind _paperflipbook (Variables|Default|GetPaperFlipbook))
  (if (not (Variables|Default|GetisBreaking))
    (Variables|Default|SetisBreaking true)
    (Sprite|SetFlipbook _paperflipbook "/Game/Assets/Items/Breakdown/Box-Breakdown.Box-Breakdown")
    (Components|Timeline|SetLooping _paperflipbook false)
    (Components|Timeline|PlayfromStart _paperflipbook)
    (Audio|PlaySound2D "/Game/Assets/Sounds/66779__kevinkace__crate-break-3.66779__kevinkace__crate-break-3" 1.0 1.0 0.1 0 0)))