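; Possessable Paper2D side-view character pawn with a special ability and interactable support.
; Tick derives state from velocity to switch flipbooks and sounds, while a one-shot ability flipbook holds its state until playback finishes.
; Possession by BP_PlayerController nudges the pawn forward in depth, shows an arrow and attaches the camera; unpossession sends it back.
; Overlaps track a BPI_Interactables target, prompting only when player-controlled and forwarding interact calls.
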(event OnFinishedPlaying(Sprite)
  (bind _sprite (Variables|Default|GetSprite))
  ;[1 1 1] Sprite Event
  (if (and (not (Class|PaperFlipbookComponent|IsLooping (Variables|Default|GetSprite))) (Utilities|IsCurrentState "NewEnumerator3"))
    (Components|Timeline|SetLooping _sprite true)
    (Sprite|SetFlipbook _sprite (Variables|Animation|GetIdleAnim))
    (Components|Timeline|PlayfromStart _sprite)
    (CallFunction|SetState "NewEnumerator0")))

(event EventBeginPlay)

(event EventInteractwithInteractable
  (if (!= (Utilities|ToObject(Interface) (Variables|Default|GetOverlappingInteractable)) 0)
    (Default|Interact (Variables|Default|GetOverlappingInteractable))))

(event EventTick
  (params (DeltaSeconds :type Float%20%28single-precision%29))
  (bind _audio (Variables|Default|GetAudio))
  (bind _audio_2 (Variables|Default|GetAudio))
  (if (Utilities|IsinAir)
    (CallFunction|SetState "NewEnumerator2")
    (CallFunction|SetJumpFallFlipbook)
    (elif (not (Utilities|IsUsingAbility))
      (if (Utilities|IsMoving)
        (Sprite|SetFlipbook (Variables|Default|GetSprite) (Variables|Animation|GetIdleAnim))
        (CallFunction|SetState "NewEnumerator0")
        (Audio|Components|Audio|Stop _audio)
        (Audio|Components|Audio|SetSound _audio 0)
        (else
          (Sprite|SetFlipbook (Variables|Default|GetSprite) (Variables|Animation|GetRunAnim))
          (CallFunction|SetState "NewEnumerator1")
          (if (!= (Variables|Sound|GetRunSound) (Variables|/Script/Engine.AudioComponent|GetSound (Variables|Default|GetAudio)))
            (Audio|Components|Audio|SetSound _audio_2 (Variables|Sound|GetRunSound))
            (Audio|Components|Audio|Play _audio_2 0.0)))))))

(event EventPossessed
  (params (NewController :type Controller%20Object%20Reference))
  (bind _overlappinginteractable (Variables|Default|GetOverlappingInteractable))
  ;[1 1 1] Possessed
  (Utilities|Casting|CastToBP_PlayerController NewController)
  (CallFunction|BringCharacterForward)
  (Rendering|SetVisibility (Variables|Default|GetPossessedArrow) true false)
  (Default|AttachtoPawn (Variables|Default|GetPlayerCamera) self)
  (if (!= (Utilities|ToObject(Interface) _overlappinginteractable) 0)
    (Default|ShowInteractPrompt _overlappinginteractable)))

(event EventLookRight
  ;[1 1 1] BPI_Flipbook
  (Transformation|SetWorldRotation (Variables|Default|GetSprite) "0, 0, 0" false false))

(event EventLookLeft
  ;[1 1 1] BPI_Flipbook
  (Transformation|SetWorldRotation (Variables|Default|GetSprite) "0,180.000000, 0" false false))

(event EventUnpossessed
  (params (OldController :type Controller%20Object%20Reference))
  (bind _overlappinginteractable (Variables|Default|GetOverlappingInteractable))
  ;[1 1 1] Possessed
  (CallFunction|SendCharacterBack)
  (Rendering|SetVisibility (Variables|Default|GetPossessedArrow) false false)
  (if (!= (Utilities|ToObject(Interface) _overlappinginteractable) 0)
    (Default|HideInteractPrompt _overlappinginteractable)))

(event EventUseAbility
  ;[1 1 1] BPI_Flipbook
  (if (!= (Variables|Animation|GetAbilityAnim) 0)
    (CallFunction|StartAbility)))

(event Collision|EventActorBeginOverlap
  (params (OtherActor :type Actor%20Object%20Reference))
  ;[1 1 1] Actor Overlap
  (CallFunction|OverlapInteractable OtherActor))

(event Collision|EventActorEndOverlap
  (params (OtherActor :type Actor%20Object%20Reference))
  ;[1 1 1] Actor Overlap
  (CallFunction|EndOverlapInteractable OtherActor))

(fn ConstructionScript)

(fn SetJumpFallFlipbook
  (bind _audio (Variables|Default|GetAudio))
  (if (Utilities|IsJumping)
    (if (and (!= (Variables|/Script/Engine.AudioComponent|GetSound (Variables|Default|GetAudio)) (Variables|Sound|GetJumpSound)) (Utilities|IsCurrentState "NewEnumerator2"))
      (Audio|Components|Audio|SetSound _audio (Variables|Sound|GetJumpSound))
      (Audio|Components|Audio|Play _audio 0.06))
    (Sprite|SetFlipbook (Variables|Default|GetSprite) (Variables|Animation|GetJumpAnim))
    (elif (Utilities|IsFalling)
      (Sprite|SetFlipbook (Variables|Default|GetSprite) (Variables|Animation|GetFallAnim))
      (Audio|Components|Audio|SetSound (Variables|Default|GetAudio) 0))))

(fn SetState
  (params (NewState :type E_CharacterState%20Enum :default "NewEnumerator0"))
  (bind _output_get (Variables|Default|SetState NewState))
  (switch Utilities|FlowControl|Switch|SwitchonE_CharacterState _output_get))

(fn BringCharacterForward
  (bind _returnvalue (Transformation|GetActorLocation))
  (Transformation|SetActorLocation (Math|Vector|MakeVector (.x _returnvalue) 0.1 (.z _returnvalue)) false false))

(fn SendCharacterBack
  (bind _returnvalue (Transformation|GetActorLocation))
  (Transformation|SetActorLocation (Math|Vector|MakeVector (.x _returnvalue) 0.0 (.z _returnvalue)) false false))

(fn StartAbility
  (bind _sprite (Variables|Default|GetSprite))
  (Components|Timeline|SetLooping _sprite false)
  (Sprite|SetFlipbook _sprite (Variables|Animation|GetAbilityAnim))
  (Components|Timeline|PlayfromStart _sprite)
  (CallFunction|SetState "NewEnumerator3"))

(fn OverlapInteractable
  (params (Object :type Object%20Object%20Reference))
  (bind _asbpi_interactables (Utilities|Casting|CastToBPI_Interactables Object))
  (Variables|Default|SetOverlappingInteractable _asbpi_interactables)
  (if (== (Pawn|GetController) (Game|GetPlayerController 0))
    (Default|ShowInteractPrompt (Variables|Default|GetOverlappingInteractable))))

(fn EndOverlapInteractable
  (params (Object :type Object%20Object%20Reference))
  (bind _asbpi_interactables (Utilities|Casting|CastToBPI_Interactables Object))
  (Default|HideInteractPrompt _asbpi_interactables)
  (Variables|Default|SetOverlappingInteractable 0))

(fn CanUseAbility
  (return (and (not (Utilities|IsinAir)) (not (Utilities|IsUsingAbility)))))

(fn IsAbilityActive
  (return (Utilities|IsUsingAbility)))