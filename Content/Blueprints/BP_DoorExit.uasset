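; Exit door interactable that ends the level once it has been unlocked.
; Unlock sets a flag that gates both interaction and the inherited show and hide of the interact prompt.
; Interacting flags the player controller as interacting, plays the gameplay camera's outro, shows an outro message widget after a short delay, then opens the named next level.
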(event EventBeginPlay
  (|CallParentFunction) ; This node is disabled and will not be called.\nDrag off pins to build functionality.
)

(event Collision|EventActorBeginOverlap
  (params (OtherActor :type Actor%20Object%20Reference))
  (|CallParentFunction OtherActor))

(event EventTick
  (params (DeltaSeconds :type Float%20%28single-precision%29))
  (|CallParentFunction DeltaSeconds) ; This node is disabled and will not be called.\nDrag off pins to build functionality.
)

(event EventInteract
  (if (Variables|Default|GetIsUnlocked)
    (bind _asbp_player_controller (Utilities|Casting|CastToBP_PlayerController (Game|GetPlayerController 0)))
    (Variables|/Game/Blueprints/BP_PlayerController.BP_PlayerController_C|SetIsInteracting _asbp_player_controller true)
    (Default|PlayOutro (Variables|Default|GetGameplayCamera))
    (Utilities|FlowControl|Delay 1.0)
    (bind _returnvalue (UserInterface|CreateWidget "/Game/Widgets/W_OutroMessage.W_OutroMessage_C" (Game|GetPlayerController 0)))
    (UserInterface|Viewport|AddtoViewport _returnvalue 0)
    (Utilities|FlowControl|Delay 3.0)
    (Game|OpenLevel(byName) (Variables|Default|GetNextLevel%20Name))))

(event EventUnlock
  (Variables|Default|SetIsUnlocked true))

(event EventHideInteractPrompt
  (if (Variables|Default|GetIsUnlocked)
    (|CallParentFunction)))

(event EventShowInteractPrompt
  (if (Variables|Default|GetIsUnlocked)
    (|CallParentFunction)))

(fn ConstructionScript
  (|CallParentFunction))