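; Magic boulder variant that carries a key for unlocking a designated object.
; On BeginPlay, after running the parent logic, it casts the KeyActor child actor to BP_Key and passes UnlockableObjectForKey into the key's UnlockableObject.
; All other behavior is left to the parent class, as the construction script only calls its parent and the Overlap and Tick events are disabled.
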(event EventBeginPlay
  (|CallParentFunction)
  (bind _asbp_key (Utilities|Casting|CastToBP_Key (Variables|/Script/Engine.ChildActorComponent|GetChildActor (Variables|Default|GetKeyActor))))
  (Variables|/Game/Blueprints/BP_Key.BP_Key_C|SetUnlockableObject _asbp_key (Variables|Default|GetUnlockableObjectForKey)))

(event Collision|EventActorBeginOverlap
  (params (OtherActor :type Actor%20Object%20Reference))
  (|CallParentFunction OtherActor) ; This node is disabled and will not be called.\nDrag off pins to build functionality.
)

(event EventTick
  (params (DeltaSeconds :type Float%20%28single-precision%29))
  (|CallParentFunction DeltaSeconds) ; This node is disabled and will not be called.\nDrag off pins to build functionality.
)

(fn ConstructionScript
  (|CallParentFunction))