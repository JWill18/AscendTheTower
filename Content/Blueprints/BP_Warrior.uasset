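; Warrior character with a flipbook sprite, whose melee ability breaks barricades in front of it.
; UseAbility runs the parent logic and plays a swoosh sound.
; Tick polls the sprite and, past 70% of the ability flipbook with the ability timer check passed, line-traces forward by AbilityRange and calls Break on a hit BP_Barricade.
; The timer increment in Tick adds zero, and nothing here resets it.
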(event EventBeginPlay)

(event Collision|EventActorBeginOverlap
  (params (OtherActor :type Actor%20Object%20Reference))
  (|CallParentFunction OtherActor) ; This node is disabled and will not be called.\nDrag off pins to build functionality.
)

(event EventTick
  (params (DeltaSeconds :type Float%20%28single-precision%29))
  (bind _returnvalue (Transformation|GetActorLocation))
  (bind _sprite (Variables|Default|GetSprite))
  (|CallParentFunction DeltaSeconds)
  ;[1 1 1] Used to prevent spawning another one before the animation ends
  (Variables|Default|SetCurrentAbilityTimer (+ (Variables|Default|GetCurrentAbilityTimer) 0.0))
  (if (and (and (== (Class|PaperFlipbookComponent|GetFlipbook _sprite) "/Game/AssetPacks/Characters/Medieval_Warrior_Pack_3/Medieval_Warrior_Pack_3/Sprites/Ability/Warrior_Ability.Warrior_Ability") (> (/ (Math|Conversions|ToFloat(Integer) (Class|PaperFlipbookComponent|GetPlaybackPositioninFrames _sprite)) (Math|Conversions|ToFloat(Integer) (Class|PaperFlipbookComponent|GetFlipbookLengthinFrames _sprite))) 0.7)) (>= (Variables|Default|GetCurrentAbilityTimer) (Variables|Default|GetAbilityTimer)))
    (bind _outhit (Collision|LineTraceByChannel _returnvalue (+ _returnvalue (* (Math|Vector|GetForwardVector (Variables|Default|GetSprite)) (Math|Vector|MakeVector (Variables|Default|GetAbilityRange) 0.0 0.0))) "TraceTypeQuery1" false 0 "None" true "(R=1.000000,G=0.000000,B=0.000000,A=1.000000)" "(R=0.000000,G=1.000000,B=0.000000,A=1.000000)" 1.0))
    (bind _asbp_barricade (Utilities|Casting|CastToBP_Barricade (.hitactor _outhit)))
    (Default|Break _asbp_barricade)))

(event EventUseAbility
  (|CallParentFunction)
  (Audio|PlaySound2D "/Game/Assets/Sounds/216675__hitrison__stick-swoosh-whoosh.216675__hitrison__stick-swoosh-whoosh" 1.0 1.0 0.0 0 0))

(fn ConstructionScript
  (|CallParentFunction))