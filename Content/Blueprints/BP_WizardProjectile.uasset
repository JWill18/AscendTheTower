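; BP_WizardProjectile is a wizard's flipbook-based spell projectile that explodes on impact and then removes itself.
; On overlap with any actor that is neither a Pawn nor another wizard projectile, it stops its ProjectileMovement, plays the explosion flipbook once and plays a fireball sound.
; The actor destroys itself when the Spell flipbook finishes playing.
; It applies no damage, and a debug print branch is left unconnected.
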(event OnFinishedPlaying(Spell)
  (Actor|DestroyActor))

(event EventBeginPlay)

(event EventTick
  (params (DeltaSeconds :type Float%20%28single-precision%29)))

(event Collision|EventActorBeginOverlap
  (params (OtherActor :type Actor%20Object%20Reference))
  (bind _returnvalue (Utilities|GetClass OtherActor))
  (bind _spell (Variables|Default|GetSpell))
  (if (and (not (Utilities|ClassIsChildOf _returnvalue "/Script/Engine.Pawn")) (not (Utilities|ClassIsChildOf _returnvalue "BP_WizardProjectile_C")))
    (Components|Movement|StopMovementImmediately (Variables|Default|GetProjectileMovement))
    (Components|Timeline|SetLooping _spell false)
    (Sprite|SetFlipbook _spell "/Game/Assets/Abilities/Wizard/Explosion/Wizard_SpellExplosion.Wizard_SpellExplosion")
    (Components|Timeline|PlayfromStart _spell)
    (Audio|PlaySound2D "/Game/Assets/Sounds/431174__highpixel__fireball-explosion.431174__highpixel__fireball-explosion" 1.0 1.0 0.0 0 0)))

(fn ConstructionScript)