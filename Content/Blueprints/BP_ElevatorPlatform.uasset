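; 2D elevator platform whose PaperSprite slides between TopPosition and BottomPosition, starting at the end chosen by Position in the construction script.
; While IsMoving, set by StartMoving and StopMoving, Tick moves it toward the opposite end; when stopped, it eases any displacement back to Position's end.
; Movement uses constant-speed VInterpToConstant, with a snap onto the target when nearly there.
; Position is never changed within this Blueprint.
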(event EventBeginPlay)

(event Collision|EventActorBeginOverlap
  (params (OtherActor :type Actor%20Object%20Reference)))

(event EventTick
  (params (DeltaSeconds :type Float%20%28single-precision%29))
  (if (and (not (Variables|Default|GetIsMoving)) (not (Utilities|PlatformatEndPoint)))
    ;[1 1 1] Reset Position if out of position
    (switch Utilities|FlowControl|Switch|SwitchonE_PlatformPosition (Variables|Default|GetPosition)
      (:NewEnumerator0
        (CallFunction|SlidetoPosition (Utilities|Time|GetWorldDeltaSeconds) (Transformation|GetWorldLocation (Variables|Default|GetTopPosition)))
        (CallFunction|ClamptoPosition (Transformation|GetWorldLocation (Variables|Default|GetTopPosition))))
      (:NewEnumerator1
        (CallFunction|SlidetoPosition (Utilities|Time|GetWorldDeltaSeconds) (Transformation|GetWorldLocation (Variables|Default|GetBottomPosition)))
        (CallFunction|ClamptoPosition (Transformation|GetWorldLocation (Variables|Default|GetBottomPosition)))))
    (elif (Variables|Default|GetIsMoving)
      (switch Utilities|FlowControl|Switch|SwitchonE_PlatformPosition (Variables|Default|GetPosition)
        (:NewEnumerator0
          (CallFunction|SlidetoPosition (Utilities|Time|GetWorldDeltaSeconds) (Transformation|GetWorldLocation (Variables|Default|GetBottomPosition)))
          (CallFunction|ClamptoPosition (Transformation|GetWorldLocation (Variables|Default|GetBottomPosition))))
        (:NewEnumerator1
          (CallFunction|SlidetoPosition (Utilities|Time|GetWorldDeltaSeconds) (Transformation|GetWorldLocation (Variables|Default|GetTopPosition)))
          (CallFunction|ClamptoPosition (Transformation|GetWorldLocation (Variables|Default|GetTopPosition))))))))

(fn ConstructionScript
  (switch Utilities|FlowControl|Switch|SwitchonE_PlatformPosition (Variables|Default|GetPosition)
    (:NewEnumerator0
      (LocalVariables|Setlocal_StartingPosition (Transformation|GetWorldLocation (Variables|Default|GetTopPosition))))
    (:NewEnumerator1
      (LocalVariables|Setlocal_StartingPosition (Transformation|GetWorldLocation (Variables|Default|GetBottomPosition)))))
  (Transformation|SetWorldLocation (Variables|Default|GetPaperSprite) (LocalVariables|Getlocal_StartingPosition) false false))

(fn ClamptoPosition
  (params (Position :type Vector))
  (if (Utilities|Operators|EqualEqual (Transformation|GetWorldLocation (Variables|Default|GetPaperSprite)) Position 0.1)
    (Transformation|SetWorldLocation (Variables|Default|GetPaperSprite) Position false false)))

(fn SlidetoPosition
  (params (DeltaTime :type Float%20%28single-precision%29) (Position :type Vector))
  (Transformation|SetWorldLocation (Variables|Default|GetPaperSprite) (Utilities|MovetoPosition DeltaTime Position) false false))

(fn StartMoving
  (Variables|Default|SetIsMoving true))

(fn StopMoving
  (Variables|Default|SetIsMoving false))