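; Gameplay camera actor that attaches to the character pawn and runs intro and outro vertical pans.
; At BeginPlay, a timeline slides it to the intro destination height, which becomes its lowest allowed Z.
; Outside pans, Tick locks X and Y to the placed position and clamps Z to that floor, leaving only vertical following.
; PlayOutro suspends the clamp and pans from the current location by a Z offset.
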(event Custom|PlayOutro
  (bind _returnvalue (Transformation|GetActorLocation))
  (Variables|Default|SetCameraPanning true)
  (Variables|Default|SetOutroStartingLocation _returnvalue)
  (Variables|Default|SetOutroDestinationLocation (+ _returnvalue (Math|Vector|MakeVector 0.0 0.0 (Variables|Default|GetOutroDestinationRange))))
  (bind _outro (Timeline|OutroPan Play)
    (:Update
      (Transformation|SetActorLocation (Math|Vector|Lerp(Vector) (Variables|Default|GetOutroStartingLocation) (Variables|Default|GetOutroDestinationLocation) _outro) false false))))

(event EventBeginPlay
  (bind _introstartinglocation (Variables|Default|GetIntroStartingLocation))
  (Variables|Default|SetCameraPanning true)
  (bind _slidein (Timeline|IntroPan Play)
    (:Update
      (Transformation|SetActorLocation (Math|Vector|Lerp(Vector) (Math|Vector|MakeVector (.x _introstartinglocation) (.y _introstartinglocation) (.z _introstartinglocation)) (Math|Vector|MakeVector (.x _introstartinglocation) (.y _introstartinglocation) (.z (Variables|Default|GetIntroDestinationLocation))) _slidein) false false))
    (:Finished
      (Variables|Default|SetLowestZPosition (.z (Transformation|GetActorLocation)))
      (Variables|Default|SetCameraPanning false))))

(event Collision|EventActorBeginOverlap
  (params (OtherActor :type Actor%20Object%20Reference)))

(event EventTick
  (params (DeltaSeconds :type Float%20%28single-precision%29))
  (bind _returnvalue (Transformation|GetActorLocation))
  (bind _introstartinglocation (Variables|Default|GetIntroStartingLocation))
  (bind _lowestzposition (Variables|Default|GetLowestZPosition))
  (if (not (Variables|Default|GetCameraPanning))
    (Transformation|SetActorLocation (Math|Vector|MakeVector (.x _introstartinglocation) (.y _introstartinglocation) (Math|Float|SelectFloat (.z _returnvalue) _lowestzposition (> (.z _returnvalue) _lowestzposition))) false false)))

(fn ConstructionScript
  (Variables|Default|SetIntroStartingLocation (Transformation|GetActorLocation)))

(fn AttachtoPawn
  (params (Pawn :type Pawn%20Object%20Reference))
  (bind _asbp_character_pawn (Utilities|Casting|CastToBP_CharacterPawn Pawn))
  (Transformation|AttachActorToActor _asbp_character_pawn "None" "KeepRelative" "KeepWorld" "KeepWorld" false))