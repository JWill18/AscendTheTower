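; BP_Interactable is an interactable object that displays an animated interaction prompt matched to the player's input device.
; On BeginPlay it binds to the BP_PlayerController's gameplay control change dispatcher, which swaps the InteractionSymbol flipbook between keyboard and gamepad icons.
; Show and hide events toggle the symbol's visibility, restarting its animation when shown; the interaction itself is not implemented here.
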(event EventBeginPlay
  (bind _asbp_player_controller (Utilities|Casting|CastToBP_PlayerController (Game|GetPlayerController 0)))
  (EventDispatchers|BindEventtoOnGameplayControlChange _asbp_player_controller (EventDispatchers|CreateEvent :!event OnGameplayControlChange)))

(event Collision|EventActorBeginOverlap
  (params (OtherActor :type Actor%20Object%20Reference)))

(event EventTick
  (params (DeltaSeconds :type Float%20%28single-precision%29)))

(event EventHideInteractPrompt
  (Rendering|SetVisibility (Variables|Default|GetInteractionSymbol) false false))

(event EventShowInteractPrompt
  (Rendering|SetVisibility (Variables|Default|GetInteractionSymbol) true false)
  (Components|Timeline|PlayfromStart (Variables|Default|GetInteractionSymbol)))

(fn ConstructionScript)

(fn OnGameplayControlChange
  (params (GameplayControls :type E_GameplayControls%20Enum :default "NewEnumerator0"))
  (bind _interactionsymbol (Variables|Default|GetInteractionSymbol))
  (switch Utilities|FlowControl|Switch|SwitchonE_GameplayControls GameplayControls
    (:NewEnumerator0
      (Sprite|SetFlipbook _interactionsymbol (Variables|Default|GetKeyboardInteractionIcon)))
    (:NewEnumerator1
      (Sprite|SetFlipbook _interactionsymbol (Variables|Default|GetGamepadInteractIcon)))))