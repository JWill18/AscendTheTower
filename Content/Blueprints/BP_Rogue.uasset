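; BP_Rogue is a 2D flipbook character that adds wall sliding and wall jumping to its parent class.
; In one State value, Tick line-traces against WorldStatic along the sprite's facing, switching to the slide flipbook on a hit.
; Slide start turns the sprite around, so later traces invert the direction to keep finding the wall.
; ApplyForce launches a sliding Rogue along its forward vector with a velocity-change impulse.
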(event EventBeginPlay
  (|CallParentFunction) ; This node is disabled and will not be called.\nDrag off pins to build functionality.
)

(event Collision|EventActorBeginOverlap
  (params (OtherActor :type Actor%20Object%20Reference))
  (|CallParentFunction OtherActor) ; This node is disabled and will not be called.\nDrag off pins to build functionality.
)

(event EventTick
  (params (DeltaSeconds :type Float%20%28single-precision%29))
  (|CallParentFunction DeltaSeconds)
  (if (Utilities|Enum|Equal(Enum) (Variables|Default|GetState) "NewEnumerator2")
    (CallFunction|CheckforWallSlide)
    (else
      (Variables|Default|SetIsWallSliding false))))

(event EventApplyForce
  (if (Variables|Default|GetIsWallSliding)
    (Physics|AddImpulse (Variables|Character|GetCharacterMovement) (* (Math|Vector|GetForwardVector (Variables|Default|GetSprite)) (Variables|Default|GetWallJumpForce)) true)
    (Variables|Default|SetIsWallSliding false)))

(fn ConstructionScript
  (|CallParentFunction))

(fn CheckforWallSlide
  (bind _returnvalue (Transformation|GetActorLocation))
  (bind _sprite (Variables|Default|GetSprite))
  (bind _direction (CallFunction|GetWallSlideDirection))
  (bind _returnvalue_2 (Collision|LineTraceForObjects _returnvalue (+ _returnvalue _direction) (Utilities|Array|MakeArray "ObjectTypeQuery1") false 0 "None" true "(R=1.000000,G=0.000000,B=0.000000,A=1.000000)" "(R=0.000000,G=1.000000,B=0.000000,A=1.000000)" 1.0))
  (if _returnvalue_2
    (Sprite|SetFlipbook _sprite "/Game/AssetPacks/Characters/Plague_Warrior/Plague_Warrior/Sprites/WallSlide/Rogue_WallSlide.Rogue_WallSlide")
    (if (not (Variables|Default|GetIsWallSliding))
      (if (!= (.yaw (Transformation|GetWorldRotation _sprite)) 0.0)
        (CallFunction|LookRight)
        (else
          (CallFunction|LookLeft)))
      (Variables|Default|SetIsWallSliding true))
    (else
      (Variables|Default|SetIsWallSliding false))))

(fn GetWallSlideDirection
  (if (Variables|Default|GetIsWallSliding)
    (LocalVariables|Setlocal_Direction (* (* (Math|Vector|GetForwardVector (Variables|Default|GetSprite)) "-1.000000,0,0.000000") (Math|Vector|MakeVector (Variables|Default|GetWallSlideRange) 0.0 0.0)))
    (else
      (LocalVariables|Setlocal_Direction (* (Math|Vector|GetForwardVector (Variables|Default|GetSprite)) (Math|Vector|MakeVector (Variables|Default|GetWallSlideRange) 0.0 0.0)))))
  (return (LocalVariables|Getlocal_Direction)))