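; BP_ElevatorButton is a pressure button that runs its linked ElevatorPlatform while a BP_CharacterPawn overlaps it.
; Each qualifying overlap increments a counter, starts the platform and hides EnvObjectsSprite2.
; When the counter drops to zero, the platform stops and the sprite reappears, so the button stays active until every pawn has left.
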(event EventBeginPlay)

(event Collision|EventActorBeginOverlap
  (params (OtherActor :type Actor%20Object%20Reference))
  (if (Utilities|ClassIsChildOf (Utilities|GetClass OtherActor) "/Game/Blueprints/BP_CharacterPawn.BP_CharacterPawn_C")
    (Math|Integer|IncrementInt (Variables|Default|GetNumOfOverlaps)
      (:%20%20
        (Default|StartMoving (Variables|Default|GetElevatorPlatform))
        (Rendering|SetVisibility (Variables|Default|Getenv_objects_Sprite_2) false false)))))

(event EventTick
  (params (DeltaSeconds :type Float%20%28single-precision%29)))

(event Collision|EventActorEndOverlap
  (params (OtherActor :type Actor%20Object%20Reference))
  (if (Utilities|ClassIsChildOf (Utilities|GetClass OtherActor) "/Game/Blueprints/BP_CharacterPawn.BP_CharacterPawn_C")
    (bind _result (Math|Integer|DecrementInt (Variables|Default|GetNumOfOverlaps))
      (:%20%20
        (if (<= _result 0)
          (Default|StopMoving (Variables|Default|GetElevatorPlatform))
          (Variables|Default|SetNumOfOverlaps 0)
          (Rendering|SetVisibility (Variables|Default|Getenv_objects_Sprite_2) true false))))))

(fn ConstructionScript)