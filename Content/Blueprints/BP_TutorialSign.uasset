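; BP_TutorialSign is an interactable sign that shows and hides a tutorial message on screen.
; BeginPlay creates the W_TutorialMessage widget with keyboard text by default.
; Interact toggles the widget in the viewport and sets IsInteracting on BP_PlayerController to match.
; An OnGameplayControlChange override swaps the text between keyboard and gamepad versions when the control scheme changes.
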(event EventBeginPlay
  (CallFunction|CreateTutorialWidget)
  (|CallParentFunction))

(event Collision|EventActorBeginOverlap
  (params (OtherActor :type Actor%20Object%20Reference))
  (|CallParentFunction OtherActor) ; This node is disabled and will not be called.\nDrag off pins to build functionality.
)

(event EventTick
  (params (DeltaSeconds :type Float%20%28single-precision%29))
  (|CallParentFunction DeltaSeconds) ; This node is disabled and will not be called.\nDrag off pins to build functionality.
)

(event EventInteract
  (bind _tutorialwidget (Variables|Default|GetTutorialWidget))
  (if (UserInterface|Viewport|IsinViewport _tutorialwidget)
    (Widget|RemovefromParent _tutorialwidget)
    (bind _asbp_player_controller (Utilities|Casting|CastToBP_PlayerController (Game|GetPlayerController 0)))
    (Variables|/Game/Blueprints/BP_PlayerController.BP_PlayerController_C|SetIsInteracting _asbp_player_controller false)
    (else
      (UserInterface|Viewport|AddtoViewport _tutorialwidget 0)
      (bind _asbp_player_controller_2 (Utilities|Casting|CastToBP_PlayerController (Game|GetPlayerController 0)))
      (Variables|/Game/Blueprints/BP_PlayerController.BP_PlayerController_C|SetIsInteracting _asbp_player_controller_2 true))))

(fn ConstructionScript
  (|CallParentFunction))

(fn OnGameplayControlChange
  (params (GameplayControls :type E_GameplayControls%20Enum :default "NewEnumerator0"))
  (bind _tutorialwidget (Variables|Default|GetTutorialWidget))
  (|CallParentFunction GameplayControls)
  (switch Utilities|FlowControl|Switch|SwitchonE_GameplayControls GameplayControls
    (:NewEnumerator0
      (Default|SetTutorialText _tutorialwidget (Variables|Default|GetKeyboardTutorialText)))
    (:NewEnumerator1
      (Default|SetTutorialText _tutorialwidget (Variables|Default|GetGamepadTutorialText)))))

(fn CreateTutorialWidget
  (bind _returnvalue (UserInterface|CreateWidget "/Game/Widgets/W_TutorialMessage.W_TutorialMessage_C" (Game|GetPlayerController 0)))
  (bind _output_get (Variables|Default|SetTutorialWidget _returnvalue))
  (Default|SetTutorialText _output_get (Variables|Default|GetKeyboardTutorialText)))